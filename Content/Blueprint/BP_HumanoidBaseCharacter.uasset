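; Base humanoid character Blueprint providing camera zoom and sprint controls.
; On BeginPlay it attaches an elemental spark particle emitter to the root component.
; Mouse wheel keys and larger-step QuickZoom actions adjust the spring arm length within clamped limits.
; Sprint doubles CharacterMovement's max walk speed on press and halves it on release, relative to the current value rather than a stored base.
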(event `self.ReceiveBeginPlay`
  (`GameplayStatics.SpawnEmitterAttached` "/Game/Particles/Elemental_Spark.Elemental_Spark" (`self.RootComponent`)))

(event `InputAction|QuickZoomUp`
  (params (Key :type "Key Structure"))
  (bind _springarmcomponent (`self.SpringArmComponent`))
  ;[1 1 1] camera zoom
  (:`Pressed`
    (set `SpringArmComponent.TargetArmLength` (`KismetMathLibrary.FClamp` (+ (`SpringArmComponent.TargetArmLength` _springarmcomponent) -200.0) 100.0 1200.0) _springarmcomponent)))

(event `InputAction|Sprint`
  (params (Key :type "Key Structure"))
  (bind _charactermovement (`self.CharacterMovement`))
  (bind _charactermovement_2 (`self.CharacterMovement`))
  ;[1 1 1] Sprint
  (:`Pressed`
    (set `CharacterMovementComponent.MaxWalkSpeed` (* (`CharacterMovementComponent.MaxWalkSpeed` _charactermovement_2) 2.0) _charactermovement_2))
  (:`Released`
    (set `CharacterMovementComponent.MaxWalkSpeed` (* (`CharacterMovementComponent.MaxWalkSpeed` _charactermovement) 0.5) _charactermovement)))

(event `Key|MouseScrollUp`
  (params (Key :type "Key Structure"))
  (bind _springarmcomponent (`self.SpringArmComponent`))
  ;[1 1 1] camera zoom
  (:`Pressed`
    (set `SpringArmComponent.TargetArmLength` (`KismetMathLibrary.FClamp` (+ (`SpringArmComponent.TargetArmLength` _springarmcomponent) -100.0) 100.0 1200.0) _springarmcomponent)))

(event `Key|MouseScrollDown`
  (params (Key :type "Key Structure"))
  (bind _springarmcomponent (`self.SpringArmComponent`))
  ;[1 1 1] camera zoom
  (:`Pressed`
    (set `SpringArmComponent.TargetArmLength` (`KismetMathLibrary.FClamp` (+ (`SpringArmComponent.TargetArmLength` _springarmcomponent) 100.0) 100.0 1200.0) _springarmcomponent)))

(event `InputAction|QuickZoomDown`
  (params (Key :type "Key Structure"))
  (bind _springarmcomponent (`self.SpringArmComponent`))
  ;[1 1 1] camera zoom
  (:`Pressed`
    (set `SpringArmComponent.TargetArmLength` (`KismetMathLibrary.FClamp` (+ (`SpringArmComponent.TargetArmLength` _springarmcomponent) 200.0) 100.0 1200.0) _springarmcomponent)))

(fn `UserConstructionScript`)